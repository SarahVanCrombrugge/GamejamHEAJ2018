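; Flag actor that loses Life while opposing soldiers stand inside its shield and is destroyed when Life runs out.
; FlagShield overlap events add or remove Soldiers whose IsEnemy differs from the flag's Enemy value in the Enemies list.
; Tick subtracts each listed soldier's DamageValue scaled by delta time, so damage stacks per attacker.
; Cube and actor rotation nodes are left unconnected.
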(event OnComponentBeginOverlap(FlagShield)
  (params (OverlappedComponent :type Primitive%20Component%20Object%20Reference) (OtherActor :type Actor%20Object%20Reference) (OtherComp :type Primitive%20Component%20Object%20Reference) (OtherBodyIndex :type Integer) (bFromSweep :type Boolean) (SweepResult :type Hit%20Result%20Structure%20%28by%20ref%29))
  ;[1 1 1] CheckCollision with soldiers
  (bind _assoldier (Utilities|Casting|CastToSoldier OtherActor))
  (if (not (Math|Boolean|Equal(Boolean) (Variables|/Game/Blueprint/Soldier.Soldier_C|GetisEnemy _assoldier) (Variables|Default|GetEnemy)))
    (Utilities|Array|Add (Variables|Default|GetEnemies) _assoldier)))

(event OnComponentEndOverlap(FlagShield)
  (params (OverlappedComponent :type Primitive%20Component%20Object%20Reference) (OtherActor :type Actor%20Object%20Reference) (OtherComp :type Primitive%20Component%20Object%20Reference) (OtherBodyIndex :type Integer))
  ;[1 1 1] CheckCollision with soldiers
  (bind _assoldier (Utilities|Casting|CastToSoldier OtherActor))
  (if (not (Math|Boolean|Equal(Boolean) (Variables|/Game/Blueprint/Soldier.Soldier_C|GetisEnemy _assoldier) (Variables|Default|GetEnemy)))
    (Utilities|Array|RemoveItem (Variables|Default|GetEnemies) _assoldier)))

(event EventTick
  (params (DeltaSeconds :type Float%20%28single-precision%29))
  ;[1 1 1] Life check
  (if (<= (Variables|Default|GetLife) 0.0)
    (Actor|DestroyActor)
    (else
      (for _array_element (Variables|Default|GetEnemies)
        (Variables|Default|SetLife (- (Variables|Default|GetLife) (* (Variables|/Game/Blueprint/Soldier.Soldier_C|GetDamageValue _array_element) DeltaSeconds)))))))

(fn ConstructionScript)