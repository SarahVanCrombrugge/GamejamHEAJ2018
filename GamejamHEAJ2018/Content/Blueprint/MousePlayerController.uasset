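; Mouse player controller that deploys soldier formations and spawns enemy legions for the game mode's current level shortly after BeginPlay.
; A left-click drag traces under the cursor, setting a friendly legion's position from the press and facing from the release.
; SpawnLegion builds a centred grid of AI Soldiers, rotating it by temporarily attaching them to a spawned Gizmo.
; Right click fires OnUnleachEnemy; the FautToutFaireSoiMemeIci rotation helper is unused.
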(event EventBeginPlay
  (Utilities|FlowControl|Delay 0.1)
  (CallFunction|SpawnEnemies))

(event EventTick
  (params (DeltaSeconds :type Float%20%28single-precision%29)))

(event Input|ActionEvents|InputActionLeftClick
  (params (Key :type Key%20Structure))
  ;[1 1 1] Mouse to pos
  (:Pressed
    (bind (_worldpos _hit) (CallFunction|GetClickPos))
    (if _hit
      (bind _output_get (Variables|Default|SetMouseWorldPos _worldpos))))
  (:Released
    (bind (_worldpos_2 _hit_2) (CallFunction|GetClickPos))
    (if _hit_2
      (if _hit
        (CallFunction|SpawnLegion 2 5 (Math|Rotator|MakeRotator 0.0 0.0 (Class|KismetMathLibrary|DegAtan2 (.Y (Math|Vector|BreakVector (- _worldpos_2 (Variables|Default|GetMouseWorldPos)))) (.X (Math|Vector|BreakVector (- _worldpos_2 (Variables|Default|GetMouseWorldPos)))))) _output_get false)))))

(event Input|MouseEvents|RightMouseButton
  (params (Key :type Key%20Structure))
  (:Pressed
    (Default|CallOnUnleachEnemy)))

(fn ConstructionScript)

(fn SpawnLegion
  (params (Line :type Integer) (Row :type Integer) (Orientation :type Rotator :default "0,0,1.000000") (Position :type Vector) (Enemy :type Boolean))
  (bind _returnvalue (- Line 1))
  (bind _returnvalue_2 (- Row 1))
  (bind _soldiers (Variables|Default|GetSoldiers))
  ;[1 1 1] Spawn and rotation
  (bind _output_get (LocalVariables|SetCenter Position))
  (Development|PrintString (Utilities|String|ToString(Vector) _output_get))
  (for _index (range 0 _returnvalue)
    (for _index_2 (range 0 _returnvalue_2)
      (bind _returnvalue_3 (AI|SpawnAIFromClass "/Game/Blueprint/Soldier.Soldier_C" 0 (+ (* (Math|Vector|MakeVector (- (Math|Conversions|ToFloat(Integer) _index) (/ (Math|Conversions|ToFloat(Integer) _returnvalue) 2.0)) (- (Math|Conversions|ToFloat(Integer) _index_2) (/ (Math|Conversions|ToFloat(Integer) _returnvalue_2) 2.0)) 0.0) 1e+02) (LocalVariables|GetCenter)) Orientation false))
      (bind _assoldier (Utilities|Casting|CastToSoldier _returnvalue_3))
      (Default|OnSpawned _assoldier self Enemy)
      (Utilities|Array|Add (Variables|Default|GetSoldiers) _assoldier)))
  (bind _returnvalue_4 (Game|SpawnActorfromClass "/Game/Blueprint/Gizmo.Gizmo_C" (Math|Conversions|ToTransform(Vector) (LocalVariables|GetCenter)) "AlwaysSpawn" 0 0))
  (for _array_element (Variables|Default|GetSoldiers)
    (Transformation|AttachActorToActor _array_element _returnvalue_4 "None" "KeepWorld" "KeepWorld" "KeepWorld" true))
  (Transformation|AddActorLocalRotation _returnvalue_4 Orientation false false) ; Ca non plus ca marche pas c'est daubé du cul.En fait si ca marche mais pas sur cet actor la visiblement
  (for _array_element_2 _soldiers
    (Transformation|DetachFromActor _array_element_2 "KeepWorld" "KeepWorld" "KeepWorld"))
  (Utilities|Array|Clear _soldiers))

(fn FautToutFaireSoiMemeIci
  (params (ObjectToRotate :type Actor%20Object%20Reference) (Point :type Vector) (Rotation :type Rotator))
  (bind _returnvalue (Game|SpawnActorfromClass "/Script/Engine.Actor" (Math|Conversions|ToTransform(Vector) Point) "AlwaysSpawn" 0 0))
  (Transformation|AttachActorToActor ObjectToRotate _returnvalue "None" "KeepRelative" "KeepRelative" "KeepRelative" true) ; Visiblement c'est de la merde et ca marche pas donc ca sert a rien
  (Transformation|AddActorLocalRotation _returnvalue Rotation false false) ; Ca non plus ca marche pas c'est daubé du cul.En fait si ca marche mais pas sur cet actor la visiblement
  (Development|PrintString "Hello"))

(fn GetClickPos
  (bind _returnvalue (Game|GetPlayerController 0))
  (bind (_worldlocation _worlddirection) (Game|Player|ConvertMouseLocationToWorldSpace _returnvalue))
  (bind (_outhit _returnvalue_2) (Collision|LineTraceByChannel _worldlocation (+ _worldlocation (* _worlddirection 1e+04)) "TraceTypeQuery1" false 0 "None"))
  (return (+ (.Location (Collision|BreakHitResult _outhit)) "0, 0,100.000000") _returnvalue_2))

(fn SpawnEnemies
  (bind _ascustom_game_mode (Utilities|Casting|CastToCustomGameMode (Game|GetGameMode)))
  (Development|PrintString (Utilities|String|ToString(Integer) (Variables|/Game/CustomGameMode.CustomGameMode_C|GetCurrentLevel _ascustom_game_mode)))
  (switch int (Variables|/Game/CustomGameMode.CustomGameMode_C|GetCurrentLevel _ascustom_game_mode)
    (:0
      (CallFunction|SpawnLegion 2 2 "0,180.000000,0.000000" "240.000000,-2110.000000,20.000000" true))
    (:1
      (CallFunction|SpawnLegion 3 3 "0,0,1.000000" "0, 0, 0" true))
    (:2
      (CallFunction|SpawnLegion 3 3 "0,0,1.000000" "0, 0, 0" true)
      (CallFunction|SpawnLegion 3 3 "0,0,1.000000" "0, 0, 0" true))
    (:3
      (CallFunction|SpawnLegion 3 3 "0,0,1.000000" "0, 0, 0" true)
      (CallFunction|SpawnLegion 3 3 "0,0,1.000000" "0, 0, 0" true)))
  (return))