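; Team-based battle soldier, tinted red or blue on spawn, that seeks opposing soldiers or the opposing team's flag.
; Tick damages every enemy inside AttackRange over time and, unless targeting a living soldier, rescans all soldiers for the closest enemy, falling back to the flag.
; Movement toward the target starts only when the mouse controller's OnUnleachEnemy event fires.
; At zero life it loses movement, launches upward as a physics body and stops ticking.
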(event OnComponentBeginOverlap(AttackRange)
  (params (OverlappedComponent :type Primitive%20Component%20Object%20Reference) (OtherActor :type Actor%20Object%20Reference) (OtherComp :type Primitive%20Component%20Object%20Reference) (OtherBodyIndex :type Integer) (bFromSweep :type Boolean) (SweepResult :type Hit%20Result%20Structure%20%28by%20ref%29))
  ;[1 1 1] AttackRange
  (if (not (== OtherActor 0))
    (bind _assoldier (Utilities|Casting|CastToSoldier OtherActor))
    (if (Math|Boolean|NotEqual(Boolean) (Variables|Soldier_C|GetisEnemy _assoldier) (Variables|Default|GetisEnemy))
      (Utilities|Array|Add (Variables|Default|GetEnemiesOnCollide) _assoldier))))

(event OnComponentEndOverlap(AttackRange)
  (params (OverlappedComponent :type Primitive%20Component%20Object%20Reference) (OtherActor :type Actor%20Object%20Reference) (OtherComp :type Primitive%20Component%20Object%20Reference) (OtherBodyIndex :type Integer))
  ;[1 1 1] AttackRange
  (bind _assoldier (Utilities|Casting|CastToSoldier OtherActor))
  (Utilities|Array|RemoveItem (Variables|Default|GetEnemiesOnCollide) _assoldier))

(event OnComponentBeginOverlap(DetectionRange)
  (params (OverlappedComponent :type Primitive%20Component%20Object%20Reference) (OtherActor :type Actor%20Object%20Reference) (OtherComp :type Primitive%20Component%20Object%20Reference) (OtherBodyIndex :type Integer) (bFromSweep :type Boolean) (SweepResult :type Hit%20Result%20Structure%20%28by%20ref%29)))

(event Custom|OnResolve
  (bind _objectif (Variables|Default|GetObjectif))
  ;[1 1 1] Move
  (Utilities|IsValid (Variables|Character|GetCharacterMovement)
    (:Is%20Valid
      (Utilities|IsValid _objectif
        (:Is%20Valid
          (AI|Navigation|SimpleMovetoActor (Pawn|GetController) _objectif))))))

(event Custom|OnSpawned
  (params (Mouse%20Controller%20ref :type Mouse%20Player%20Controller%20Object%20Reference) (isEnemy :type Boolean))
  (bind _sphere (Variables|Default|GetSphere))
  ;[1 1 1] On spawned setup
  (bind _output_get (Variables|Default|SetisEnemy isEnemy))
  (if _output_get
    (Rendering|Material|SetVectorParameterValueonMaterials _sphere "DefaultColor" "1.000000, 0, 0")
    (else
      (Rendering|Material|SetVectorParameterValueonMaterials _sphere "DefaultColor" "0.000000,0.000000,1.000000")))
  (bind _output_get_2 (Variables|Default|SetMouseRef Mouse%20Controller%20ref))
  (EventDispatchers|AssignOnUnleachEnemy _output_get_2 (delegate Custom|OnResolve))
  (bind _outactors (Actor|GetAllActorsOfClass "/Game/Blueprint/Flag.Flag_C"))
  (bind _array_element (Utilities|Array|ForEachLoopwithBreak _outactors :!label _label)
    (:LoopBody
      (if (Variables|Default|GetisEnemy)
        (if (not (Variables|/Game/Blueprint/Flag.Flag_C|GetEnemy _array_element))
          (Variables|Default|SetObjectif _array_element :!label _label_2)
          (goto _label Break))
        (elif (Variables|/Game/Blueprint/Flag.Flag_C|GetEnemy _array_element)
          (goto _label_2))))
    (:Completed
      (Class|CharacterMovementComponent|SetAvoidanceEnabled (Variables|Character|GetCharacterMovement) true))))

(event EventTick
  (params (DeltaSeconds :type Float%20%28single-precision%29))
  (bind _enemiesoncollide (Variables|Default|GetEnemiesOnCollide))
  ;[1 1 1] Check life
  (if (<= (Variables|Default|GetLife) 0.0)
    (Variables|Default|SetisAlive false)
    (Components|DestroyComponent (Variables|Character|GetCharacterMovement))
    ;[1 1 1] Death
    (Physics|SetSimulatePhysics (Variables|Collision|GetCapsuleComponent) true)
    (Physics|AddForce (Variables|Collision|GetCapsuleComponent) "0, 0,100000.000000" "None" true)
    (Actor|Tick|SetActorTickEnabled false)
    (else
      ;[1 1 1] Attack
      (for _array_element _enemiesoncollide
        (if (Utilities|IsValid _array_element)
          (Variables|Soldier_C|SetLife _array_element (- (Variables|Soldier_C|GetLife _array_element) (* (Variables|Default|GetDamageValue) DeltaSeconds)))
          (else
            (Utilities|Array|RemoveItem _enemiesoncollide _array_element))))
      (Utilities|IsValid (Variables|Default|GetObjectif)
        (:Is%20Valid
          (bind _assoldier (Utilities|Casting|CastToSoldier (Variables|Default|GetObjectif))
            (:then
              (if (not (Variables|Soldier_C|GetisAlive _assoldier))
                (bind _outactors (Actor|GetAllActorsOfClass "Soldier_C" :!label _label))
                (bind _array_element_2 (Utilities|Array|ForEachLoopwithBreak _outactors)
                  (:LoopBody
                    (if (<= (Math|Vector|VectorLengthSquared (- (Transformation|GetActorLocation _array_element_2) (Transformation|GetActorLocation))) (Variables|Default|GetMinDist))
                      (if (Math|Boolean|NotEqual(Boolean) (Variables|Default|GetisEnemy) (Variables|Soldier_C|GetisEnemy _array_element_2))
                        (Variables|Default|SetMinDist (Math|Vector|VectorLengthSquared (- (Transformation|GetActorLocation _array_element_2) (Transformation|GetActorLocation))))
                        (bind _output_get (Variables|Default|SetClosestEnemy _array_element_2)))))
                  (:Completed
                    (Utilities|IsValid _output_get
                      (:Is%20Valid
                        (Variables|Default|SetObjectif _output_get))
                      (:Is%20Not%20Valid
                        ;[1 1 1] On spawned setup
                        (bind _outactors_2 (Actor|GetAllActorsOfClass "/Game/Blueprint/Flag.Flag_C"))
                        (bind _array_element_3 (Utilities|Array|ForEachLoopwithBreak _outactors_2 :!label _label_2)
                          (:LoopBody
                            (if (Variables|Default|GetisEnemy)
                              (if (not (Variables|/Game/Blueprint/Flag.Flag_C|GetEnemy _array_element_3))
                                (Variables|Default|SetObjectif _array_element_3 :!label _label_3)
                                (goto _label_2 Break))
                              (elif (Variables|/Game/Blueprint/Flag.Flag_C|GetEnemy _array_element_3)
                                (goto _label_3))))
                          (:Completed
                            (Class|CharacterMovementComponent|SetAvoidanceEnabled (Variables|Character|GetCharacterMovement) true)))))))))
            (:CastFailed
              (goto _label))))
        (:Is%20Not%20Valid
          (goto _label))))))

(fn ConstructionScript)